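; BP_openDoor is a door that swings open or closed when the player presses E near it.
; Box overlap begin and end enable and disable input for player controller 0, without checking which actor overlaps.
; On E, the DoorRotation timeline plays if its current value is below 1, otherwise reverses, driving the door's relative yaw through about 90 degrees.
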(event OnComponentBeginOverlap(Box)
  (params (OverlappedComponent :type Primitive%20Component%20Object%20Reference) (OtherActor :type Actor%20Object%20Reference) (OtherComp :type Primitive%20Component%20Object%20Reference) (OtherBodyIndex :type Integer) (bFromSweep :type Boolean) (SweepResult :type Hit%20Result%20Structure%20%28by%20ref%29))
  ;[1 1 1] open door by pressing E inside collision box
  (Input|EnableInput (Game|GetPlayerController 0)) ; pressing E will open the door
)

(event OnComponentEndOverlap(Box)
  (params (OverlappedComponent :type Primitive%20Component%20Object%20Reference) (OtherActor :type Actor%20Object%20Reference) (OtherComp :type Primitive%20Component%20Object%20Reference) (OtherBodyIndex :type Integer))
  ;[1 1 1] open door by pressing E inside collision box
  (Input|DisableInput (Game|GetPlayerController 0)) ; pressing E will no longer open the door
)

(event Input|KeyboardEvents|E
  (params (Key :type Key%20Structure :default "AnyKey"))
  ;[1 1 1] open door by pressing E inside collision box
  (:Pressed
    (if (< (stale _doorrotation) 1.0) ; if rotation of door < 1 (if door is closed)
      (bind _doorrotation (Timeline|doorRotation Play) ; timeline that takes 2.25 seconds to change door's rotation by 90 degrees
        (:Update
          (Transformation|SetRelativeRotation (Variables|Default|Getdoor) (Math|Rotator|MakeRotator 0.0 0.0 _doorrotation) false false) ; set rotation of door
        ))
      (else
        (Timeline|doorRotation Reverse)))))

(fn ConstructionScript)