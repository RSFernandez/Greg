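; Terminal is an interactable Blueprint that toggles the player's view between the first-person character and a linked camera.
; On Interact while inactive, it switches player 0's view target to CorrespondingCamera, marks itself active and ignores move and look input.
; On Interact while active, it loops over all FirstPersonCharacter actors to set the view back, clears the active flag and resets the input-ignore flags.
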(event EventInteract
  (bind _returnvalue (Game|GetPlayerController 0))
  (if (Variables|Default|GetIsActive)
    (bind _outactors (Actor|GetAllActorsOfClass "/Game/FirstPersonBP/Blueprints/FirstPersonCharacter.FirstPersonCharacter_C"))
    (for _array_element _outactors
      (Game|Player|SetViewTargetwithBlend (Game|GetPlayerController 0) _array_element 0.0 "VTBlend_Linear" 0.0 false)
      (Variables|Default|SetIsActive false)
      (Class|Controller|ResetIgnoreInputFlags (Game|GetPlayerController 0)))
    (else
      (Game|Player|SetViewTargetwithBlend (Game|GetPlayerController 0) (Variables|Default|GetCorrespondingCamera) 0.0 "VTBlend_Linear" 0.0 false)
      (bind _output_get (Variables|Default|SetIsActive true))
      (Input|SetIgnoreMoveInput _returnvalue _output_get)
      (Input|SetIgnoreLookInput _returnvalue _output_get))))

(fn ConstructionScript)