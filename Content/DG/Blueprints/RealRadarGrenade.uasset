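; A radar grenade that marks Sentinels inside its detection sphere with red radar dots and destroys itself after 15 seconds.
; Every Tick it hides all Sentinel meshes from the minimap camera's scene capture.
; While an overlap flag is set by begin/end overlap events, Tick also spawns a new dot actor at each overlapping Sentinel's location.
; ShowOnRadar and a duplicate hide function are defined but never called here.
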(event EventBeginPlay
  ;[1 1 1] Destroys Grenade
  (Variables|Default|SetisOverlap false)
  (Utilities|FlowControl|Delay 15.0)
  (Actor|DestroyActor))

(event EventTick
  (params (DeltaSeconds :type Float%20%28single-precision%29))
  (bind _detection_sphere (Variables|Default|GetDetection%20Sphere))
  (bind _overlappingactors (Collision|GetOverlappingActors _detection_sphere "/Game/DG/AI/Sentinel.Sentinel_C" :!class /Script/Engine.PrimitiveComponent))
  ;[1 1 1] Checks for overlapping sentinels, then makes them visible or invisible on the radar if they are detected by the radar grenade
  (CallFunction|HideSentinelfromRadar)
  (if (Variables|Default|GetisOverlap)
    ;[1 1 1] Tracks locations of overlapping AI. Change the class filter to change the actor tracked.
    (for _index (range 0 (Utilities|Array|Length _overlappingactors))
      (Game|SpawnActorfromClass "/Game/DG/Blueprints/RedRadarDot_Blueprint.RedRadarDot_Blueprint_C" (Math|Conversions|ToTransform(Vector) (Transformation|GetActorLocation (Utilities|Array|Get(acopy) _overlappingactors _index))) "Undefined" 0 0))))

(event Collision|EventActorBeginOverlap
  (params (OtherActor :type Actor%20Object%20Reference))
  ;[1 1 1] Checks for overlapping sentinels, then makes them visible or invisible on the radar if they are detected by the radar grenade
  (Variables|Default|SetisOverlap true))

(event Collision|EventActorEndOverlap
  (params (OtherActor :type Actor%20Object%20Reference))
  ;[1 1 1] Checks for overlapping sentinels, then makes them visible or invisible on the radar if they are detected by the radar grenade
  (Variables|Default|SetisOverlap false))

(fn ConstructionScript)

(fn HideSentinelfromRadar
  (bind _outactors (Actor|GetAllActorsOfClass "/Game/DG/AI/Sentinel.Sentinel_C"))
  (for _index (range 0 (Utilities|Array|Length _outactors))
    (bind _outactors_2 (Actor|GetAllActorsOfClass "/Game/doorAndTrapsBP/BP_miniMapCamera.BP_miniMapCamera_C"))
    (Class|SceneCaptureComponent|HideComponent (Variables|/Script/Engine.SceneCapture2D|GetCaptureComponent2D (Utilities|Array|Get(acopy) _outactors_2)) (Variables|/Script/Engine.Character|GetMesh (Utilities|Array|Get(acopy) _outactors _index)))))

(fn ShowonRadar
  (bind _outactors (Actor|GetAllActorsOfClass "/Game/ThirdPersonBP/Blueprints/AI.AI_C"))
  (for _index (range 0 (Utilities|Array|Length _outactors))
    (bind _outactors_2 (Actor|GetAllActorsOfClass "/Game/doorAndTrapsBP/BP_miniMapCamera.BP_miniMapCamera_C"))
    (bind _asai (Utilities|Casting|CastToAI (Utilities|Array|Get(acopy) _outactors)))
    (Rendering|SetVisibility (Variables|/Script/Engine.Character|GetMesh _asai) true true)))

(fn HideSentinelfromRadar0
  (bind _outactors (Actor|GetAllActorsOfClass "/Game/DG/AI/Sentinel.Sentinel_C"))
  (for _index (range 0 (Utilities|Array|Length _outactors))
    (bind _outactors_2 (Actor|GetAllActorsOfClass "/Game/doorAndTrapsBP/BP_miniMapCamera.BP_miniMapCamera_C"))
    (Class|SceneCaptureComponent|HideComponent (Variables|/Script/Engine.SceneCapture2D|GetCaptureComponent2D (Utilities|Array|Get(acopy) _outactors_2)) (Variables|/Script/Engine.Character|GetMesh (Utilities|Array|Get(acopy) _outactors _index)))))