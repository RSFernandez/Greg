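; ColorDoor is a key-locked door that slides open when the player interacts while holding the matching key.
; Interact compares the first-person character's held key to the door's required key and calls Open on a match.
; Open plays the DoorSlide timeline, setting the actor's location to its BeginPlay start position plus the timeline's offset, and prints debug strings.
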(event Custom|Open
  (Development|PrintString "opening")
  (bind _doorslide (Timeline|DoorSlide Play)
    (:Update
      (Transformation|SetActorLocation (+ _doorslide (Variables|Default|GetStartPosition)) false false))
    (:Finished
      (Development|PrintString "opened"))))

(event EventBeginPlay
  (Variables|Default|SetStartPosition (Transformation|GetActorLocation)))

(event Collision|EventActorBeginOverlap
  (params (OtherActor :type Actor%20Object%20Reference)))

(event EventTick
  (params (DeltaSeconds :type Float%20%28single-precision%29)))

(event EventInteract
  (bind _asfirst_person_character (Utilities|Casting|CastToFirstPersonCharacter (Game|Player|GetPlayerPawn 0)))
  (if (Utilities|Enum|Equal(Enum) (Variables|/Game/FirstPersonBP/Blueprints/FirstPersonCharacter.FirstPersonCharacter_C|GetkeyHeld _asfirst_person_character) (Variables|Default|GetKeyRequired))
    (CallFunction|Open)))

(fn ConstructionScript)