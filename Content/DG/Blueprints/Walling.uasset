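; Walling is a Blueprint that moves a set of wall actors, apparently raising them, when its Trigger event fires.
; BeginPlay writes a WallsLocation entry for each wall, with no location value wired in.
; Trigger plays a timeline whose WallGoesUp track is added to each entry, scaled by LocationMultiplier and applied as an unswept local offset.
; The offset is relative and applied every timeline update, so movement accumulates.
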(event EventBeginPlay
  ;[1 1 1] Set The Local Location
  (for (_ _array_index) (Variables|Default|GetWalls)
    (Utilities|Array|SetArrayElem (Variables|Default|GetWallsLocation) _array_index "")))

(event EventTrigger
  ;[1 1 1] Add z to the location
  (bind _wallgoesup (Timeline|Timeline_0 Play)
    (:Update
      (for (_array_element _array_index) (Variables|Default|GetWalls)
        (Transformation|AddActorLocalOffset _array_element (* (+ (Utilities|Array|Get(acopy) (Variables|Default|GetWallsLocation) _array_index) _wallgoesup) (Variables|Default|GetLocationMultiplier)) false false)))))

(fn ConstructionScript
  (|CallParentFunction))