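; HUD Blueprint for a chatbox system that creates the main HUD widget and relays incoming chat messages.
; On BeginPlay it adds W_MainHud to the viewport and gives it a reference back to this HUD.
; It then retries the PS_ChatboxTut player state cast every second until it succeeds and binds to its received-message event.
; Each received message is rebroadcast with its sender through the HUD's OnChatMessageRcvd dispatcher.
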(event Custom|RcvdChatMsg
  (params (ChatSender :type Text) (ChatMessage :type Text))
  (Default|CallOnChatMessageRcvd ChatSender ChatMessage))

(event EventBeginPlay
  (bind _returnvalue (Game|Player|GetOwningPlayerController))
  (bind _returnvalue_2 (UserInterface|CreateWidget "/Game/UI/W_MainHud.W_MainHud_C" _returnvalue))
  (bind _output_get (Variables|Default|SetW_MainHud _returnvalue_2))
  (Variables|/Game/UI/W_MainHud.W_MainHud_C|SetourHUD _output_get self)
  (UserInterface|Viewport|AddtoViewport _returnvalue_2 10)
  (bind _asps_chatbox_tut (Utilities|Casting|CastToPS_ChatboxTut (Variables|/Script/Engine.Controller|GetPlayerState _returnvalue) :!label _label)
    (:then
      (EventDispatchers|BindEventtoRecievedAChatMessage _asps_chatbox_tut (delegate Custom|RcvdChatMsg)))
    (:CastFailed
      (Utilities|FlowControl|Delay 1.0)
      (goto _label))))

(fn ConstructionScript)